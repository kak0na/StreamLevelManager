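; BP_SwitchLevelInvoker is a debug-key test driver for the stream level manager's load, unload and switch functions.
; Numpad keys alternate odd/even DataAsset presets with custom overrides, switch hardcoded level sets, or unload all then toggle every BP_SubInvoker after a delay.
; P prints current stream levels.
; Completion is reported through a notify target (itself or a BP_InterfaceNotifyReceiver) or delegates, though the step-counting delegate's binding is disconnected.
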(event Custom|OnLoadUnloadFInished
  (params (bIsLoadCommand :type Boolean))
  ;[1 1 1] 使用多播委托
  (Development|PrintString (Utilities|String|SelectString "Load Commands Finished" "Unload Commands Finished" bIsLoadCommand))
  (bind _result (Math|Integer|DecrementInt (Variables|Default|GetStepCount))
    (:%20%20
      (if (== _result 0)
        (EventDispatchers|UnbindEventfromOnTrySwitchLevelFinished (Subsystems|GetMyStreamLevelManager) (delegate Custom|OnLoadUnloadFInished))
        (Development|PrintString "All Command Finished Unbind Delegate")))))

(event Custom|AllFinished
  ;[1 1 1] 调用场景内5个触发器的切换行为
  (Development|PrintString "All Command Finished" true true "(R=0.000000,G=0.660000,B=1.000000,A=1.000000)" 2e+01))

(event EventBeginPlay
  (bind _returnvalue (Actor|GetActorOfClass "/StreamLevelManager/Blueprint/BP_InterfaceNotifyReceiver.BP_InterfaceNotifyReceiver_C"))
  (Variables|Default|SetReceiver _returnvalue))

(event Collision|EventActorBeginOverlap
  (params (OtherActor :type Actor%20Object%20Reference)))

(event EventTick
  (params (DeltaSeconds :type Float%20%28single-precision%29)))

(event EventTrySwitchFinished
  (params (bIsLoadCommand :type Boolean))
  (Development|PrintString "Load Commands Finished,Told By Interface"))

(event Input|KeyboardEvents|DebugKeyNumPadTwo
  (params (Key :type Key%20Structure :default "None") (ActionValue :type Input%20Action%20Value%20Structure))
  (bind _set (Utilities|Set|MakeSet "StreamLevel1" "StreamLevel3" "StreamLevel5" "StreamLevel2"))
  (bind _set_2 (Utilities|Set|MakeSet "StreamLevel1" "StreamLevel4" "StreamLevel6"))
  (:Pressed
    (bind _isa (Utilities|FlowControl|FlipFlop)
      (:A
        _)
      (:B
        _))
    ;[1 1 1] 统一函数
    (Class|MyStreamLevelManager|SwitchLevelsinOneFunc (Subsystems|GetMyStreamLevelManager) (select _isa _set_2 _set) (select _isa _set _set_2) (Variables|Default|GetReceiver))))

(event Input|KeyboardEvents|DebugKeyP
  (params (Key :type Key%20Structure :default "None") (ActionValue :type Input%20Action%20Value%20Structure))
  (:Pressed
    ;[1 1 1] 打印当前已加载的关卡名称
    (bind _result (Utilities|Set|ToArray (Class|MyStreamLevelManager|GetCurrentStreamLevels (Subsystems|GetMyStreamLevelManager))))
    (for _array_element _result
      (Development|PrintString (Utilities|String|ToString(Name) _array_element)))))

(event Input|KeyboardEvents|DebugKeyNumPadOne
  (params (Key :type Key%20Structure :default "None") (ActionValue :type Input%20Action%20Value%20Structure))
  (bind _returnvalue (Subsystems|GetMyStreamLevelManager))
  (:Pressed
    ;[1 1 1] 卸载所有关卡
    (Class|MyStreamLevelManager|TryUnloadSomeLevels _returnvalue (Class|MyStreamLevelManager|GetCurrentStreamLevels _returnvalue) self)
    (Utilities|FlowControl|Delay 5.0)
    ;[1 1 1] 调用场景内5个触发器的切换行为
    (EventDispatchers|BindEventtoSwitchAllStreamLevelFinished (Subsystems|GetMyStreamLevelManager) (delegate Custom|AllFinished))
    (bind _outactors (Actor|GetAllActorsOfClass "/StreamLevelManager/Blueprint/BP_SubInvoker.BP_SubInvoker_C"))
    (for _array_element _outactors
      (Default|ToggleGivenLevelsStreamState _array_element))))

(event Input|KeyboardEvents|DebugKeyNumPadZero
  (params (Key :type Key%20Structure :default "None") (ActionValue :type Input%20Action%20Value%20Structure))
  (:Pressed
    ;[1 1 1] 在预设的基础上额外附加关卡加卸载，用户附加关卡优先级高于预设
    ;;[1 1 1] 偶数编号、奇数编号交替
    (bind _isa (Utilities|FlowControl|FlipFlop)
      (:A
        _)
      (:B
        _))
    (Variables|Default|SetbShowEvenIndex _isa)
    (bind _returnvalue (Utilities|LoadClassAssetBlocking (.Value (Utilities|Map|Find (Variables|Default|GetPresetNameToDataAsset) (select (Variables|Default|GetbShowEvenIndex) (Utilities|Name|MakeLiteralName "Even") (Utilities|Name|MakeLiteralName "Odd"))))))
    (bind _asda_level_perset (Utilities|Casting|CastToDA_LevelPersetClass _returnvalue))
    (bind _returnvalue_2 (Game|ConstructObjectfromClass _asda_level_perset))
    (bind (_levelstoload _levelstoremove) (Default|GetPresetLevels _returnvalue_2))
    (Class|MyStreamLevelManager|LoadwithPresetInfo (Subsystems|GetMyStreamLevelManager) _levelstoload _levelstoremove (select (Variables|Default|GetbShowEvenIndex) (Utilities|Set|MakeSet "StreamLevel9") (Utilities|Set|MakeSet "StreamLevel10")) (select (Variables|Default|GetbShowEvenIndex) (Utilities|Set|MakeSet "StreamLevel10") (Utilities|Set|MakeSet "StreamLevel9")) (Variables|Default|GetReceiver))))

(fn ConstructionScript)